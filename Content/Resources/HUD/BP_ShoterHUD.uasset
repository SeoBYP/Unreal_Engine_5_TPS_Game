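; Shooter HUD that draws the player's dynamic weapon crosshair at screen center.
; It caches the survivor character pawn on BeginPlay, re-acquiring it during DrawHUD if invalid.
; Each frame it draws five textures from the equipped weapon, pushing the top, bottom, left and right pieces outward by the character's spread multiplier times a maximum spread, while the middle piece stays fixed.
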(event `self.ReceiveBeginPlay`
  ;[1 1 1] Get Reference Surviver Character
  (`/Engine/EditorBlueprintResources/StandardMacros.IsValid` (`self.SurviverCharacter`)
    (:`Is Not Valid`
      (bind _asbp_suviver_character (cast `/Game/Resources/Characters/BP_SuviverCharacter` (`GameplayStatics.GetPlayerPawn` 0)))
      (set `self.SurviverCharacter` _asbp_suviver_character))))

(event `self.ReceiveDrawHUD`
  (params (SizeX :type Integer) (SizeY :type Integer))
  (bind (_x _y) (`KismetMathLibrary.BreakVector2D` (`self.CrosshairBaseCenter`)))
  (bind (_x_2 _y_2) (`KismetMathLibrary.BreakVector2D` (`self.CrosshairBaseCenter`)))
  (bind (_x_3 _y_3) (`KismetMathLibrary.BreakVector2D` (`self.CrosshairBaseCenter`)))
  (bind (_x_4 _y_4) (`KismetMathLibrary.BreakVector2D` (`self.CrosshairBaseCenter`)))
  (bind (_x_5 _y_5) (`KismetMathLibrary.BreakVector2D` (`self.CrosshairBaseCenter`)))
  (bind (_x_6 _y_6) (`KismetMathLibrary.BreakVector2D` (`self.CrosshairLocation`)))
  (bind (_x_7 _y_7) (`KismetMathLibrary.BreakVector2D` (`self.ScreenCenter`)))
  (set `self.ScreenCenter` (`KismetMathLibrary.MakeVector2D` (`KismetMathLibrary.Conv_IntToDouble` (/ SizeX 2)) (`KismetMathLibrary.Conv_IntToDouble` (/ SizeY 2))))
  (set `self.CrosshairLocation` (`KismetMathLibrary.MakeVector2D` _x_7 _y_7))
  (`/Engine/EditorBlueprintResources/StandardMacros.IsValid` (`self.SurviverCharacter`)
    (:`Is Valid`
      _)
    (:`Is Not Valid`
      (bind _asbp_suviver_character (cast `/Game/Resources/Characters/BP_SuviverCharacter` (`GameplayStatics.GetPlayerPawn` 0)))
      (set `self.SurviverCharacter` _asbp_suviver_character)))
  (set `self.CrosshairSpreadMultiplier` (`UnrealSuviverGameCharacter.GetCrosshairSpreadMultiplier` (`self.SurviverCharacter`)))
  (set `self.CrosshairBaseCenter` (`KismetMathLibrary.MakeVector2D` (- _x_6 (`self.CrosshairHalfWidth`)) (- _y_6 (`self.CrosshairHalfHeight`))))
  (`self.DrawTexture` (`Weapon.CrosshairsBottom` (`UnrealSuviverGameCharacter.EquippedWeapon` (`self.SurviverCharacter`))) _x_2 (+ _y_2 (* (`self.CrosshairSpreadMultiplier`) (`self.CrosshairSpreaMax`))) 64.0 64.0 0.0 0.0 1.0 1.0)
  (`self.DrawTexture` (`Weapon.CrosshairsTop` (`UnrealSuviverGameCharacter.EquippedWeapon` (`self.SurviverCharacter`))) _x_3 (- _y_3 (* (`self.CrosshairSpreadMultiplier`) (`self.CrosshairSpreaMax`))) 64.0 64.0 0.0 0.0 1.0 1.0)
  (`self.DrawTexture` (`Weapon.CrosshairsLeft` (`UnrealSuviverGameCharacter.EquippedWeapon` (`self.SurviverCharacter`))) (- _x_4 (* (`self.CrosshairSpreadMultiplier`) (`self.CrosshairSpreaMax`))) _y_4 64.0 64.0 0.0 0.0 1.0 1.0)
  (`self.DrawTexture` (`Weapon.CrosshairsRight` (`UnrealSuviverGameCharacter.EquippedWeapon` (`self.SurviverCharacter`))) (+ _x_5 (* (`self.CrosshairSpreadMultiplier`) (`self.CrosshairSpreaMax`))) _y_5 64.0 64.0 0.0 0.0 1.0 1.0)
  (`self.DrawTexture` (`Weapon.CrosshairsMiddle` (`UnrealSuviverGameCharacter.EquippedWeapon` (`self.SurviverCharacter`))) _x _y 64.0 64.0 0.0 0.0 1.0 1.0))

(fn `UserConstructionScript`)
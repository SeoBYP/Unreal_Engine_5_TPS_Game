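; Player character Blueprint that quits the game on Escape and provides a check for whether the character is inside an interior.
; InteriorCheck multi-traces the Visibility channel from just below the capsule's center to far overhead, looking for a hit component whose display name contains "InteriorCheck".
; As an optimization, the trace runs only when the referenced environment controller is valid and allows particles.
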(event `Key|Escape`
  (params (Key :type "Key Structure"))
  ;[1 0.3311 0] Quit Game
  (:`Pressed`
    (`KismetSystemLibrary.QuitGame` null "Quit")))

(event `self.ReceiveBeginPlay`)

(event `self.ReceiveTick`
  (params (DeltaSeconds :type "Float (single-precision)")))

(fn `InteriorCheck`
  (returns (Inside :type Boolean))
  (locals (LocalIsFound :type Boolean))
  (bind _environmentcontrollerref (`self.EnvironmentControllerRef`))
  (bind _x (.x (`SceneComponent.K2_GetComponentLocation` (`self.CapsuleComponent`))))
  (bind _y (.y (`SceneComponent.K2_GetComponentLocation` (`self.CapsuleComponent`))))
  (bind _z (.z (`SceneComponent.K2_GetComponentLocation` (`self.CapsuleComponent`))))
  ;[1 1 1] (Optimization) Use only when Allow Particles is enabled
  (`/Engine/EditorBlueprintResources/StandardMacros.IsValid` _environmentcontrollerref
    (:`Is Valid`
      (if (`/Game/PostCity/Blueprints/Controllers/BP_EnvironmentController.AllowParticles` _environmentcontrollerref)
        (bind (_outhits _returnvalue) (`KismetSystemLibrary.LineTraceMulti` (`KismetMathLibrary.MakeVector` _x _y (+ _z -20.0)) (`KismetMathLibrary.MakeVector` _x _y (+ _z 5000.0)) "TraceTypeQuery1" false (`|MakeArray` self :!type "Actor Object Reference")))
        (if _returnvalue
          (for _array_element _outhits
            (if (`KismetStringLibrary.Contains` (`KismetSystemLibrary.GetDisplayName` (`.HitComponent` (`GameplayStatics.BreakHitResult` _array_element))) "InteriorCheck")
              (set `local.LocalIsFound` true)
              (break)))
          (else
            (set `local.LocalIsFound` false)))
        (return (`local.LocalIsFound`))))))

(fn `UserConstructionScript`)
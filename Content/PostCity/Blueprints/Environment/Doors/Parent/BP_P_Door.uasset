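; Parent door Blueprint that swings a door between 0 and 90 degrees of yaw when activated, unless locked.
; The construction script poses the door from DoorValue, and BeginPlay derives the open/close direction from it.
; Activate seeks the DoorOpening timeline to match DoorValue, then plays or reverses it to drive RotateDoor.
; UpdateDoorValues stores lock state, color and name, while SetDoorStatus is an empty event.
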(event `SetDoorStatus`)

(event `self.ReceiveBeginPlay`
  (bind (_relativerotation_roll _relativerotation_pitch _relativerotation_yaw) (`KismetMathLibrary.BreakRotator` (`SceneComponent.RelativeRotation` (`self.Door`))))
  ;[1 1 1] Set Initial Values
  (set `self.RelativeYaw` _relativerotation_yaw)
  (if (> (`self.DoorValue`) 0.5)
    (set `self.Open` false)
    (else
      (set `self.Open` true))))

(event `/Game/PostCity/Blueprints/Buildings/Parent/BI_LevelObjectInteraction.Activate`
  ;[1 1 1] Open/Close Door if not Locked
  (if (not (`self.IsLocked`))
    (`TimelineComponent.SetNewTime` (`self.DoorOpening`) (`KismetMathLibrary.MapRangeClamped` (`self.DoorValue`) 0.0 1.0 0.0 2.0))
    (if (`self.Open`)
      (bind (_direction _dooropeningalpha) (`Timeline|DoorOpening` :!label _label)
        (:`Update`
          (`self.RotateDoor` _dooropeningalpha))
        (:`Finished`
          (if (> (`self.DoorValue`) 0.5)
            (set `self.Open` false)
            (else
              (set `self.Open` true)))))
      (else
        (goto _label :!via `Reverse`)))))

(event `RotateDoor`
  (params (DoorValue :type "Float (double-precision)"))
  ;[1 1 1] Rotate Door
  (`SceneComponent.K2_SetRelativeRotation` (`self.Door`) (`KismetMathLibrary.MakeRotator` 0.0 0.0 (`KismetMathLibrary.Lerp` 0.0 90.0 DoorValue)) false false)
  (set `self.DoorValue` DoorValue))

(fn `UpdateDoorValues`
  (params (IsLocked :type Boolean) (DoorColor :type "LinearColor Structure") (DoorName :type Text))
  (set `self.IsLocked` IsLocked)
  (set `self.DoorColor` DoorColor)
  (set `self.DoorName` DoorName))

(fn `UserConstructionScript`
  ;[1 1 1] Initial Door Rotation
  (`SceneComponent.K2_SetRelativeRotation` (`self.Door`) (`KismetMathLibrary.MakeRotator` 0.0 0.0 (`KismetMathLibrary.Lerp` 0.0 90.0 (`self.DoorValue`))) false false))
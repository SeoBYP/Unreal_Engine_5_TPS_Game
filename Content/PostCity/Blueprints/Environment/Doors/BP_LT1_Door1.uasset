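; BP_LT1_Door1 is a child door Blueprint for the environment that swings a single Door1 component through a quarter turn.
; It overrides RotateDoor, calling the parent and then mapping the incoming DoorValue to Door1's relative yaw with a Lerp.
; The construction script applies the same mapping to DoorValue, so the placed door's rotation reflects that value before play.
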(event `self.ReceiveBeginPlay`
  (`parent.ReceiveBeginPlay`))

(event `self.RotateDoor`
  (params (DoorValue :type "Float (double-precision)"))
  (`parent.RotateDoor` DoorValue)
  (`SceneComponent.K2_SetRelativeRotation` (`self.Door1`) (`KismetMathLibrary.MakeRotator` 0.0 0.0 (`KismetMathLibrary.Lerp` 0.0 -90.0 DoorValue)) false false))

(fn `UserConstructionScript`
  (`parent.UserConstructionScript`)
  (`SceneComponent.K2_SetRelativeRotation` (`self.Door1`) (`KismetMathLibrary.MakeRotator` 0.0 0.0 (`KismetMathLibrary.Lerp` 0.0 -90.0 (`self.DoorValue`))) false false))